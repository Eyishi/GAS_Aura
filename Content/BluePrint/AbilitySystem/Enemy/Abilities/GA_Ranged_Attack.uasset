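; Enemy ranged attack gameplay ability, currently without any projectile spawning or damage logic.
; On activation it turns the avatar toward its combat target through the combat interface, then plays a random tagged attack montage.
; It starts waiting for that montage's gameplay event and immediately queries the combat socket location for the tag, leaving the result unused.
; The ability ends only when the montage completes; interruption and cancellation are unhandled.
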(event `self.K2_ActivateAbility`
  (bind _returnvalue (`self.GetAvatarActorFromActorInfo`))
  (bind _returnvalue_2 (message `EnemyInterface.GetCombatTarget` _returnvalue))
  (bind _ascombat_interface (cast `CombatInterface` _returnvalue))
  (`CombatInterface.UpdateFacingTarget` _ascombat_interface (`Actor.K2_GetActorLocation` _returnvalue_2))
  (bind _returnvalue_3 (message `CombatInterface.GetAttackMontages` (`self.GetAvatarActorFromActorInfo`)))
  (bind _output_get (set `self.Tagged Montage` (`self.GetRandomTaggedMontageFromArray` _returnvalue_3)))
  (bind (_montage _montagetag) (break `TaggedMontage` _output_get))
  (`AbilityTask_PlayMontageAndWait.CreatePlayMontageAndWaitProxy` "None" _montage
    (:`then`
      (`AbilityTask_WaitGameplayEvent.WaitGameplayEvent` _montagetag null
        (:`then`
          (message `CombatInterface.GetCombatSocketLocation` (`self.GetAvatarActorFromActorInfo`) _montagetag))))
    (:`OnCompleted`
      (`self.K2_EndAbility`))))